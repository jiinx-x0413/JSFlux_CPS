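; BP_PC is the player controller Blueprint that bootstraps the CPS main UI and its data requests.
; On BeginPlay it constructs an HTTP object plus widget and actor manager objects, giving both managers a reference back to itself.
; It creates WBP_Main and passes it and its popup widget to the widget manager.
; It then requests hierarchy data, followed by main data after a fixed half-second delay.
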(event EventBeginPlay
  (CallFunction|ConstructObjects)
  (CallFunction|CreateMainUI)
  (Class|CPSController|RequestData "HIERARCHY")
  (Utilities|FlowControl|Delay 0.5)
  (Class|CPSController|RequestData "GETMAIN"))

(fn ConstructionScript)

(fn ConstructObjects
  (Utilities|FlowControl|Sequence
    (:then_0
      (bind _returnvalue (Game|ConstructObjectfromClass "/Script/CPS_JSFlux.HttpObject"))
      (Variables|Default|SetHttpObject _returnvalue))
    (:then_1
      (bind _returnvalue_2 (Game|ConstructObjectfromClass "/Game/CPS/Blueprints/BP_WidgetManager.BP_WidgetManager_C"))
      (bind _output_get (Variables|Default|SetWidgetManager _returnvalue_2))
      (Variables|/Script/CPS_JSFlux.CPSWidgetManager|SetPCRef _output_get self))
    (:then_2
      (bind _returnvalue_3 (Game|ConstructObjectfromClass "/Game/CPS/Blueprints/BP_ActorManager.BP_ActorManager_C"))
      (bind _output_get_2 (Variables|Default|SetActorManager _returnvalue_3))
      (Variables|/Script/CPS_JSFlux.CPSActorManager|SetPCRef _output_get_2 self))))

(fn CreateMainUI
  (bind _returnvalue (UserInterface|CreateWidget "/Game/CPS/UMG/WBP_Main.WBP_Main_C"))
  (Variables|Default|SetMainUIRef _returnvalue)
  (UserInterface|Viewport|AddtoViewport _returnvalue 0)
  (Variables|Default|SetPopupWidgetRef (Variables|/Game/CPS/UMG/WBP_Main.WBP_Main_C|GetWBP_PopupWidget _returnvalue))
  (Utilities|IsValid (Variables|Default|GetWidgetManager)
    (:Is%20Valid
      (bind _asbp_widget_manager (Utilities|Casting|CastToBP_WidgetManager (Variables|Default|GetWidgetManager))
        (:then
          (Variables|/Game/CPS/Blueprints/BP_WidgetManager.BP_WidgetManager_C|SetMainUIRef _asbp_widget_manager (Variables|Default|GetMainUIRef))
          (Variables|/Game/CPS/Blueprints/BP_WidgetManager.BP_WidgetManager_C|SetPopupWidgetRef _asbp_widget_manager (Variables|Default|GetPopupWidgetRef)))
        (:CastFailed
          (Development|PrintString "cast to Widget Manager failed at pc"))))
    (:Is%20Not%20Valid
      (Development|PrintString "Widget Manager Reference InValid"))))