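; BP_WidgetManager is a widget manager Blueprint that fills the sidebar of the main UI with button and view trees.
; It overrides two functions, one pushing HDataArray as the button tree and the other pushing VCMDataArray as the view tree to WBPSidebar through MainUIRef.
; Each override then calls its parent implementation and returns that result.
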(fn CreateButtonTreetoUI
  (Default|PushTreeButtontoSB (Variables|/Game/CPS/UMG/WBP_Main.WBP_Main_C|GetWBP_Sidebar (Variables|Default|GetMainUIRef)) (Variables|Default|GetHDataArray))
  (bind _targetarray (|CallParentFunction))
  (return _targetarray))

(fn CreateViewTreetoUI
  (Default|PushTreeViewtoSB (Variables|/Game/CPS/UMG/WBP_Main.WBP_Main_C|GetWBP_Sidebar (Variables|Default|GetMainUIRef)) (Variables|Default|GetVCMDataArray))
  (bind _targetarray (|CallParentFunction))
  (return _targetarray))